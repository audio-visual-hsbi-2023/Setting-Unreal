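; BP_OSCIn is an OSC receiver that drives left and right target actors from incoming position data, apparently Kinect tracking.
; BeginPlay starts a listening OSC server and binds a handler for received bundles.
; The handler reads only each bundle's first message, routing it by /left or /right address.
; Floats are remapped by swapping Y and Z, rotated 90 degrees, scaled by KinectPosAdj, and set as the target's relative location.
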(event Custom|OnBundleReceived
  (params (Bundle :type OSC%20Bundle%20Structure%20%28by%20ref%29) (IPAddress :type String) (Port :type Integer))
  (bind _kinectposadj (Variables|Default|GetKinectPosAdj))
  (bind _returnvalue (Class|OSCManager|GetMessagefromBundle Bundle))
  (bind _returnvalue_2 (Class|OSCManager|GetOSCMessageAddress _returnvalue))
  (bind _returnvalue_3 (Class|OSCManager|GetOSCAddressFullPath _returnvalue_2))
  (switch string _returnvalue_3
    (:/left
      (bind _values (Class|OSCManager|GetAllFloats _returnvalue))
      (Transformation|SetActorRelativeLocation (Variables|Default|GetTarget_L) (* (Math|Vector|RotateVectorAroundAxis (Math|Conversions|ToVector(Vector4) (Math|Vector4|MakeVector4 (Utilities|Array|Get(acopy) _values) (Utilities|Array|Get(acopy) _values 2) (Utilities|Array|Get(acopy) _values 1) 0.0)) 9e+01 "0.000000,0.500000,1.000000") _kinectposadj)))
    (:/right
      (bind _values_2 (Class|OSCManager|GetAllFloats _returnvalue))
      (Transformation|SetActorRelativeLocation (Variables|Default|GetTarget_R) (* _kinectposadj (Math|Vector|RotateVectorAroundAxis (Math|Conversions|ToVector(Vector4) (Math|Vector4|MakeVector4 (Utilities|Array|Get(acopy) _values_2) (Utilities|Array|Get(acopy) _values_2 2) (Utilities|Array|Get(acopy) _values_2 1) 0.0)) 9e+01 "0.000000,0.500000,1.000000"))))))

(event EventBeginPlay
  (bind _returnvalue (Class|OSCManager|CreateOSCServer (Variables|Default|GetReceive%20IPAddress) (Variables|Default|GetPort) false true "UE_OSC" 0))
  (bind _output_get (Variables|Default|SetServer _returnvalue))
  (EventDispatchers|BindEventtoOnOscBundleReceived _output_get (delegate Custom|OnBundleReceived)))

(fn ConstructionScript)